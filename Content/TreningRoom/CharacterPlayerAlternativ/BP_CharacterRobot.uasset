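; BP_CharacterRobot is a robot character Blueprint in the TreningRoom folder that serves as a test bed for animation playback.
; Pressing E plays the robot walk montage on the character mesh from its "Run" section.
; Unconnected leftover chains try single-animation playback with a timed return to Animation Blueprint mode, and a skeleton run montage replayed after a delay.
; BeginPlay, overlap, Tick and the construction script are empty.
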(event EventBeginPlay)

(event Collision|EventActorBeginOverlap
  (params (OtherActor :type Actor%20Object%20Reference)))

(event EventTick
  (params (DeltaSeconds :type Float%20%28single-precision%29)))

(event Input|KeyboardEvents|E
  (params (Key :type Key%20Structure :default "None"))
  (:Pressed
    (Animation|Montage|PlayMontage (Variables|Character|GetMesh) "/Game/TreningRoom/CharacterPlayerAlternativ/Animation/MontagAnimation/AM_RobotThirdPersonWalk_Montage.AM_RobotThirdPersonWalk_Montage" 1.0 0.0 "Run")))

(event Input|KeyboardEvents|Q
  (params (Key :type Key%20Structure :default "None")))

(fn ConstructionScript)