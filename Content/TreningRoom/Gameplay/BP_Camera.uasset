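; Training-room spy camera turret that sweeps back and forth, then tracks and fires at the player's BP_CharacterDodgeRock on sight.
; A self-restarting timeline drives the 180-degree yaw patrol while Tick runs a debug-drawn box trace from the muzzle point.
; Detection stops the patrol and unpauses looping timers for yaw-only interpolated aiming and spawning BP_BulletTurret with an explosion effect.
; Losing the player pauses both timers and, via DoOnce, resumes patrol from the current rotation.
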(event Custom|EventLookAtToPlayer
  (bind _spycameramesh (Variables|Default|GetSpyCameraMesh))
  (bind _returnvalue (Transformation|GetWorldRotation _spycameramesh))
  (bind _asbp_character_dodge_rock (Utilities|Casting|CastToBP_CharacterDodgeRock (Game|GetPlayerCharacter 0)))
  (Transformation|SetWorldRotation _spycameramesh (Math|Interpolation|RInterpTo (Math|Rotator|MakeRotator (.roll _returnvalue) (.pitch _returnvalue) (.yaw _returnvalue)) (Math|Rotator|MakeRotator (.roll _returnvalue) (.pitch _returnvalue) (+ (.yaw (Math|Rotator|FindLookatRotation (Transformation|GetActorLocation self) (Transformation|GetActorLocation _asbp_character_dodge_rock))) 9e+01)) (Utilities|Time|GetWorldDeltaSeconds) 5.0) false true))

(event Custom|EventStartLookToPlayer
  (Utilities|Time|UnpauseTimerbyHandle (Variables|Default|GetTimerLookAt)))

(event Custom|EventPauseLookToPlayer
  (Utilities|Time|PauseTimerbyHandle (Variables|Default|GetTimerLookAt)))

(event Custom|EventOnShoot
  (bind _point (Variables|Default|GetPoint))
  (bind _returnvalue (Transformation|GetWorldTransform _point))
  (Game|SpawnActorfromClass "/Game/DodgeRock/Gameplay/Turets/BP_BulletTurret.BP_BulletTurret_C" (Math|Transform|MakeTransform (.location _returnvalue) (.rotation _returnvalue) (.scale _returnvalue)) "AdjustIfPossibleButAlwaysSpawn" 0 1.0 0)
  (Effects|SpawnEmitteratLocation "/Game/Developers/Timur/Collections/ContentPack/StarterContent/Particles/P_Explosion.P_Explosion" (.location _returnvalue)))

(event Custom|EventStartPatrol
  (bind _rotationvalue (Timeline|RotationController PlayFromStart)
    (:Update
      (Transformation|SetWorldRotation (Variables|Default|GetSpyCameraMesh) (Math|Rotator|Lerp(Rotator) (Variables|Default|GetCurrentRotation) (Variables|Default|GetTargetRotation) _rotationvalue) false false))
    (:Finished
      (switch Utilities|FlowControl|Switch|SwitchonETimelineDirection (Variables|Default|GetDirection)
        (:Forward
          (Variables|Default|SetDirection "Backward")
          (Variables|Default|SetTargetRotation (Variables|Default|GetStartRotation))
          (Variables|Default|SetCurrentRotation (Variables|Default|GetEndRotation)))
        (:Backward
          (Variables|Default|SetDirection "Forward")
          (Variables|Default|SetTargetRotation (Variables|Default|GetEndRotation))
          (Variables|Default|SetCurrentRotation (Variables|Default|GetStartRotation))))
      (CallFunction|EventStartPatrol))))

(event Custom|EventStopPatrol
  (bind _rotationvalue (Timeline|RotationController Stop)
    (:Update
      (Transformation|SetWorldRotation (Variables|Default|GetSpyCameraMesh) (Math|Rotator|Lerp(Rotator) (Variables|Default|GetCurrentRotation) (Variables|Default|GetTargetRotation) _rotationvalue) false false))
    (:Finished
      (switch Utilities|FlowControl|Switch|SwitchonETimelineDirection (Variables|Default|GetDirection)
        (:Forward
          (Variables|Default|SetDirection "Backward")
          (Variables|Default|SetTargetRotation (Variables|Default|GetStartRotation))
          (Variables|Default|SetCurrentRotation (Variables|Default|GetEndRotation)))
        (:Backward
          (Variables|Default|SetDirection "Forward")
          (Variables|Default|SetTargetRotation (Variables|Default|GetEndRotation))
          (Variables|Default|SetCurrentRotation (Variables|Default|GetStartRotation))))
      (CallFunction|EventStartPatrol))))

(event EventBeginPlay
  (bind _spycameramesh (Variables|Default|GetSpyCameraMesh))
  (bind _returnvalue (Transformation|GetWorldRotation _spycameramesh))
  (Utilities|FlowControl|Sequence
    (:then_0
      (bind _returnvalue_2 (Utilities|Time|SetTimerbyEvent (EventDispatchers|CreateEvent :!event Custom|EventLookAtToPlayer) 0.01 true))
      (bind _output_get (Variables|Default|SetTimerLookAt _returnvalue_2))
      (Utilities|Time|PauseTimerbyHandle _output_get))
    (:then_1
      (bind _output_get_2 (Variables|Default|SetStartRotation _returnvalue))
      (bind _output_get_3 (Variables|Default|SetEndRotation (Math|Rotator|MakeRotator (.roll _output_get_2) (.pitch _output_get_2) (+ (.yaw _output_get_2) 1.8e+02))))
      (Variables|Default|SetCurrentRotation _returnvalue)
      (Variables|Default|SetTargetRotation _output_get_3)
      (CallFunction|EventStartPatrol))
    (:then_2
      (bind _returnvalue_3 (Utilities|Time|SetTimerbyEvent (EventDispatchers|CreateEvent :!event Custom|EventOnShoot) 0.3 true))
      (bind _output_get_4 (Variables|Default|SetCotrollerShoot _returnvalue_3))
      (Utilities|Time|PauseTimerbyHandle _output_get_4))))

(event EventTick
  (params (DeltaSeconds :type Float%20%28single-precision%29))
  (bind _bisplayer (CallFunction|LineTraceLogic))
  (if _bisplayer
    (CallFunction|EventStopPatrol)
    (CallFunction|EventStartLooktoPlayer)
    (Utilities|Time|UnpauseTimerbyHandle (Variables|Default|GetCotrollerShoot))
    (goto _label Reset)
    (else
      (Utilities|FlowControl|DoOnce false :!label _label
        (:Completed
          (Variables|Default|SetTargetRotation (Variables|Default|GetEndRotation))
          (Variables|Default|SetCurrentRotation (Transformation|GetWorldRotation (Variables|Default|GetSpyCameraMesh)))
          (Variables|Default|SetDirection "Forward")
          (CallFunction|EventPauseLooktoPlayer)
          (CallFunction|EventStartPatrol)
          (Utilities|Time|PauseTimerbyHandle (Variables|Default|GetCotrollerShoot)))))))

(fn ConstructionScript)

(fn LineTraceLogic
  (bind _point (Variables|Default|GetPoint))
  (bind _returnvalue (Transformation|GetWorldLocation _point))
  (bind (_outhit _returnvalue_2) (Collision|BoxTraceByChannel _returnvalue (+ _returnvalue (* (Math|Vector|GetForwardVector _point) 1000)) "40.000000,40.000000,40.000000" "0, 0, 0" "TraceTypeQuery3" false 0 "ForOneFrame" true "(R=1.000000,G=0.000000,B=0.000000,A=1.000000)" "(R=0.000000,G=1.000000,B=0.000000,A=1.000000)" 1e+01))
  (if _returnvalue_2
    (Utilities|Casting|CastToBP_CharacterDodgeRock (.hitactor _outhit)
      (:then
        (Variables|Default|SetStateCamera "NewEnumerator1")
        (return true))
      (:CastFailed
        (Variables|Default|SetStateCamera "NewEnumerator0")
        (return false)))
    (else
      (Variables|Default|SetStateCamera "NewEnumerator0")
      (return false))))