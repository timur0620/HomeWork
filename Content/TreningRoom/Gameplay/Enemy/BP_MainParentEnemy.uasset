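; BP_MainParentEnemy is a parent enemy Blueprint that moves toward the player and carries an on-screen UI widget.
; An event issues AIMoveTo at the dodge-rock player character, and BeginPlay starts a looping one-second timer.
; A helper sets visibility of the WBP_EnemyUI bar, aim and icon.
; A timeline animates a target enemy's aim image by scaling, spinning and tinting it, stopping on finish or on request.
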(event Custom|EventOnAnimStart
  (params (TargetAim :type BP%20Main%20Parent%20Enemy%20Object%20Reference))
  (bind _imageaimtarget (CallFunction|GetImageAim TargetAim))
  (CallFunction|EventonStopAnim)
  (Utilities|IsValid _imageaimtarget
    (:Is%20Valid
      (bind (_direction _scalevalue _colorvalue) (Timeline|ScalingAimTarget Play)
        (:Update
          (Widget|Transform|SetRenderScale _imageaimtarget (Math|Vector2D|MakeVector2D (.x (Math|Vector|Lerp(Vector) "1.000000,1.000000,1.000000" "3.000000,3.000000,3.000000" _scalevalue)) (.y (Math|Vector|Lerp(Vector) "1.000000,1.000000,1.000000" "3.000000,3.000000,3.000000" _scalevalue))))
          (Class|Widget|SetRenderTransformAngle _imageaimtarget (Math|Float|Lerp 0.0 3.6e+02 _scalevalue))
          (Appearance|SetColorandOpacity _imageaimtarget _colorvalue :!class /Script/UMG.Image))
        (:Finished
          (CallFunction|EventonStopAnim))))))

(event Custom|EventOnAIMoveToPlayer
  (bind _asbp_character_dodge_rock (Utilities|Casting|CastToBP_CharacterDodgeRock (Game|GetPlayerCharacter 0)))
  (AI|AIMoveTo self "0, 0, 0" _asbp_character_dodge_rock 1.0 false))

(event Custom|EventOnStopAnim
  (bind (_direction _scalevalue _colorvalue) (Timeline|ScalingAimTarget Stop)
    (:Update
      (Widget|Transform|SetRenderScale (CallFunction|GetImageAim (stale Custom|EventOnAnimStart TargetAim)) (Math|Vector2D|MakeVector2D (.x (Math|Vector|Lerp(Vector) "1.000000,1.000000,1.000000" "3.000000,3.000000,3.000000" _scalevalue)) (.y (Math|Vector|Lerp(Vector) "1.000000,1.000000,1.000000" "3.000000,3.000000,3.000000" _scalevalue))))
      (Class|Widget|SetRenderTransformAngle (CallFunction|GetImageAim (stale Custom|EventOnAnimStart TargetAim)) (Math|Float|Lerp 0.0 3.6e+02 _scalevalue))
      (Appearance|SetColorandOpacity (CallFunction|GetImageAim (stale Custom|EventOnAnimStart TargetAim)) _colorvalue :!class /Script/UMG.Image))
    (:Finished
      (CallFunction|EventonStopAnim))))

(event EventBeginPlay
  (Utilities|Time|SetTimerbyEvent (EventDispatchers|CreateEvent :!event Custom|EventOnAIMoveToPlayer) 1.0 true))

(event Collision|EventActorBeginOverlap
  (params (OtherActor :type Actor%20Object%20Reference)))

(event EventTick
  (params (DeltaSeconds :type Float%20%28single-precision%29)))

(fn ConstructionScript)

(fn GetandViewWidgetEnemy
  (params (bVisibleBar :type Boolean) (bVisibleAim :type Boolean) (bVisibleIcon :type Boolean))
  (bind _aswbp_enemy_ui (Utilities|Casting|CastToWBP_EnemyUI (UserInterface|GetWidget (Variables|Default|GetWidgetAimEnemyMain))))
  (Default|ViewUiEnemyController _aswbp_enemy_ui bVisibleBar bVisibleAim bVisibleIcon)
  (return _aswbp_enemy_ui))

(fn GetImageAim
  (params (TargetAim :type BP%20Main%20Parent%20Enemy%20Object%20Reference))
  (bind _aswbp_enemy_ui (Utilities|Casting|CastToWBP_EnemyUI (UserInterface|GetWidget (Variables|BP_MainParentEnemy_C|GetWidgetAimEnemyMain TargetAim))))
  (return (Variables|/Game/TreningRoom/Gameplay/UI/Widgets/WBP_EnemyUI.WBP_EnemyUI_C|GetImageAimTarget _aswbp_enemy_ui)))