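; BP_HomingBomb is a bomb that stays dormant until Activate is called, then launches itself at the player.
; A looping timer, paused while inactive, drives a check that grows the collision sphere as the player gets closer.
; At maximum scale it explodes upward, takes one delayed impulse toward the player, then self-destructs.
; Overlapping an actor tagged Player applies damage, then spawns an explosion and destroys it after a delay.
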(event Custom|EventCheckDistanceImpulsAtack
  (bind _returnvalue (Utilities|GetClampedDistance))
  (if (< _returnvalue (Variables|Default|GetMaxScale))
    (Transformation|SetWorldScale3D (Variables|Default|GetSphereCollision) (Math|Vector|MakeVector _returnvalue _returnvalue _returnvalue))
    (else
      (Utilities|ImpulsUp)
      (Utilities|FlowControl|Delay 0.5)
      (Utilities|ImpulstoPlayer)
      (Utilities|FlowControl|Delay 1.0)
      (Utilities|IsValid self
        (:Is%20Valid
          (Actor|DestroyActor))))))

(event EventBeginPlay
  (Utilities|FlowControl|Sequence
    (:then_0
      (bind _returnvalue (Utilities|Time|SetTimerbyEvent (EventDispatchers|CreateEvent :!event Custom|EventCheckDistanceImpulsAtack) 0.05 true))
      (Variables|Default|SetTimerCheckDistance _returnvalue)
      (CallFunction|Deactivate))))

(event EventActivate
  (Utilities|Time|UnpauseTimerbyHandle (Variables|Default|GetTimerCheckDistance))
  (Variables|/Script/Engine.PrimitiveComponent|SetbGenerateOverlapEvents (Variables|Default|GetSphereCollision) true))

(event EventDeactivate
  (Utilities|Time|PauseTimerbyHandle (Variables|Default|GetTimerCheckDistance))
  (Variables|/Script/Engine.PrimitiveComponent|SetbGenerateOverlapEvents (Variables|Default|GetSphereCollision) false))

(event Collision|EventActorBeginOverlap
  (params (OtherActor :type Actor%20Object%20Reference))
  (bind _returnvalue (Transformation|GetActorTransform))
  (if (Actor|ActorHasTag OtherActor "Player")
    (Game|Damage|ApplyDamage OtherActor 1e+01 0 self)
    (Utilities|FlowControl|Delay 1.0)
    (Effects|SpawnEmitteratLocation "/Game/Developers/Timur/Collections/ContentPack/StarterContent/Particles/P_Explosion.P_Explosion" (.location _returnvalue) (.rotation _returnvalue) (.scale _returnvalue))
    (Actor|DestroyActor)))

(fn ConstructionScript)