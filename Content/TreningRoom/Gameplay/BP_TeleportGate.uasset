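; BP_TeleportGate is a gate that teleports the player to another gate of its class.
; Its Init event stores all gates in BP_GameStateDodgeRock's Teleports array.
; On Player-tagged overlap, it disables every gate mesh's collision, flags itself as Start and moves the player to each non-Start gate, ending at the last, keeping rotation and scale.
; A one-second delay then restores mesh collision.
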(event Collision|EventActorBeginOverlap
  (params (OtherActor :type Actor%20Object%20Reference))
  (bind _returnvalue (Game|GetPlayerCharacter 0))
  (bind _gamestatedodgerock (Variables|Default|GetGameStateDodgeRock))
  (bind _returnvalue_2 (Transformation|GetActorTransform _returnvalue))
  (bind _teleports (Variables|/Game/DodgeRock/Core/GameState/BP_GameStateDodgeRock.BP_GameStateDodgeRock_C|GetTeleports _gamestatedodgerock))
  (if (Actor|ActorHasTag OtherActor "Player")
    (for _array_element _teleports
      (Collision|SetCollisionEnabled (Variables|BP_TeleportGate_C|GetStaticMeshGate _array_element) "NoCollision")
      (Variables|BP_TeleportGate_C|SetbStart _array_element false))
    (Variables|Default|SetbStart true)
    (for _array_element_2 _teleports
      (if (not (Variables|BP_TeleportGate_C|GetbStart _array_element_2))
        (Transformation|SetActorTransform _returnvalue (Math|Transform|MakeTransform (.location (Transformation|GetActorTransform _array_element_2)) (.rotation _returnvalue_2) (.scale _returnvalue_2)) false true)
        (Utilities|FlowControl|Delay 1.0)
        (for _array_element_3 (Variables|/Game/DodgeRock/Core/GameState/BP_GameStateDodgeRock.BP_GameStateDodgeRock_C|GetTeleports (Variables|Default|GetGameStateDodgeRock))
          (Collision|SetCollisionEnabled (Variables|BP_TeleportGate_C|GetStaticMeshGate _array_element_3) "QueryAndPhysics"))))))

(event EventInit
  (bind _outactors (Actor|GetAllActorsOfClass "BP_TeleportGate_C"))
  (bind _asbp_game_state_dodge_rock (Utilities|Casting|CastToBP_GameStateDodgeRock (Game|GetGameState)))
  (Variables|/Game/DodgeRock/Core/GameState/BP_GameStateDodgeRock.BP_GameStateDodgeRock_C|SetTeleports _asbp_game_state_dodge_rock _outactors)
  (Variables|Default|SetGameStateDodgeRock _asbp_game_state_dodge_rock))

(fn ConstructionScript)