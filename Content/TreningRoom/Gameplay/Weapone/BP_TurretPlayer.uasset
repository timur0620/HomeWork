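; Player turret that scales in on activation, tracks BP_MainParentEnemy actors inside a detection sphere and can fire BP_BulletTurret from its muzzle.
; Sphere overlaps maintain the enemy list, target and enemy widgets, with target cycling and a timeline return when none remain.
; Looping timers, paused at start, are toggled by Activate/Deactivate for aim interpolation and a debug-only line trace; the shoot timer is never unpaused here.
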(event OnComponentBeginOverlap(SphereDetectedCollision)
  (params (OverlappedComponent :type Primitive%20Component%20Object%20Reference) (OtherActor :type Actor%20Object%20Reference) (OtherComp :type Primitive%20Component%20Object%20Reference) (OtherBodyIndex :type Integer) (bFromSweep :type Boolean) (SweepResult :type Hit%20Result%20Structure%20%28by%20ref%29))
  (bind _asbp_main_parent_enemy (Utilities|Casting|CastToBP_MainParentEnemy OtherActor))
  (Default|GetandViewWidgetEnemy _asbp_main_parent_enemy true false true)
  (Utilities|Array|AddUnique (Variables|Default|GetEnemyes) _asbp_main_parent_enemy)
  (Utilities|FlowControl|DoOnce false
    (:Completed
      (Variables|Default|SetTargetAim _asbp_main_parent_enemy))))

(event OnComponentEndOverlap(SphereDetectedCollision)
  (params (OverlappedComponent :type Primitive%20Component%20Object%20Reference) (OtherActor :type Actor%20Object%20Reference) (OtherComp :type Primitive%20Component%20Object%20Reference) (OtherBodyIndex :type Integer))
  (bind _asbp_main_parent_enemy (Utilities|Casting|CastToBP_MainParentEnemy OtherActor))
  (Default|GetandViewWidgetEnemy _asbp_main_parent_enemy false false false)
  (Utilities|Array|RemoveItem (Variables|Default|GetEnemyes) _asbp_main_parent_enemy)
  (if (Utilities|Array|ContainsItem (Variables|Default|GetEnemyes) (Variables|Default|GetTargetAim))
    _
    (else
      (CallFunction|EventonNextTarget)))
  (if (== (Utilities|Array|Length (Variables|Default|GetEnemyes)) 0)
    (CallFunction|EventonClearAllAim)
    (Utilities|FlowControl|DoOnce false) ; enters at Reset
  ))

(event Custom|EventOnClearAllAim
  (bind _outactors (Actor|GetAllActorsOfClasswithTag "/Game/TreningRoom/Gameplay/Enemy/BP_MainParentEnemy.BP_MainParentEnemy_C" "Enemy"))
  (for _array_element _outactors
    (Default|EventonStopAnim _array_element))
  (CallFunction|EventonReternStandartPositionTurret)
  (Variables|Default|SetTargetAim 0))

(event Custom|EventOnReternStandartPositionTurret
  (bind _turretmesh (Variables|Default|GetTurretMesh))
  (bind _reternvalua (Timeline|RotatorTurret PlayFromStart)
    (:Update
      (Transformation|SetRelativeTransform _turretmesh (Math|Transform|MakeTransform "0, 0, 0" (Math|Rotator|Lerp(Rotator) (Transformation|GetWorldRotation _turretmesh) "0, 0, 0" _reternvalua) (Variables|Default|GetCurrentScale)) false false))))

(event Custom|EventOnLookToTarget
  (bind _targetaim (Variables|Default|GetTargetAim))
  (bind _turretmesh (Variables|Default|GetTurretMesh))
  (Utilities|IsValid _targetaim
    (:Is%20Valid
      (Transformation|SetWorldRotation _turretmesh (Math|Interpolation|RInterpTo (Transformation|GetWorldRotation _turretmesh) (Math|Rotator|FindLookatRotation (Transformation|GetWorldLocation _turretmesh) (Transformation|GetActorLocation _targetaim)) (Utilities|Time|GetWorldDeltaSeconds) 5.0) false false))))

(event Custom|EventOnLineTrace
  (bind _muzzleshoot (Variables|Default|GetMuzzleShoot))
  (bind _returnvalue (Transformation|GetWorldLocation _muzzleshoot))
  (Collision|LineTraceByChannel _returnvalue (+ _returnvalue (* (Math|Vector|GetForwardVector _muzzleshoot) 1000)) "TraceTypeQuery3" false 0 "ForOneFrame"))

(event Custom|EventOnNextTarget
  (bind (_lenchenemys _indextarget) (CallFunction|GetLenchEnemysandTargetIndex true true))
  (bind (_lenchenemys_2 _indextarget_2) (CallFunction|GetLenchEnemysandTargetIndex true true))
  (if (>= _lenchenemys_2 _indextarget_2)
    (if (== _lenchenemys _indextarget)
      (Variables|Default|SetTargetAim (Utilities|Array|Get(acopy) (Variables|Default|GetEnemyes)))
      (CallFunction|EventonAimVisible false)
      (else
        (bind _result (Math|Integer|IncrementInt _indextarget)
          (:%20%20
            (Variables|Default|SetTargetAim (Utilities|Array|Get(acopy) (Variables|Default|GetEnemyes) _result))
            (CallFunction|EventonAimVisible false)))))))

(event Custom|EventOnShoot
  (Game|SpawnActorfromClass "/Game/DodgeRock/Gameplay/Turets/BP_BulletTurret.BP_BulletTurret_C" (Transformation|GetWorldTransform (Variables|Default|GetMuzzleShoot)) "AdjustIfPossibleButAlwaysSpawn" 0 1.0 0))

(event Custom|EventOnAimVisible
  (params (bInVisibilAll :type Boolean))
  (bind _targetaim (Variables|Default|GetTargetAim))
  (for _array_element (Variables|Default|GetEnemyes)
    (Utilities|IsValid _array_element
      (:Is%20Valid
        (Default|GetandViewWidgetEnemy _array_element true false true)
        (Default|EventonStopAnim _array_element))))
  (if (not bInVisibilAll)
    (Utilities|IsValid _targetaim
      (:Is%20Valid
        (Default|GetandViewWidgetEnemy _targetaim true true true)
        (Default|EventonAnimStart _targetaim _targetaim)))))

(event Custom|EventOnStartAnimActivation
  (bind _scalevalue (Timeline|ScalingWeapon PlayFromStart)
    (:Update
      (Utilities|FlowControl|Sequence
        (:then_0
          (Transformation|SetWorldScale3D (Variables|Default|GetSphereDetectedCollision) (Math|Vector|Lerp(Vector) "0, 0, 0" "30.000000,30.000000,30.000000" _scalevalue)))
        (:then_1
          (Transformation|SetWorldScale3D (Variables|Default|GetTurretMesh) (Math|Vector|Lerp(Vector) "0, 0, 0" "1.000000,1.000000,1.000000" _scalevalue))
          (Variables|Default|SetCurrentScale (Math|Vector|Lerp(Vector) "0, 0, 0" "1.000000,1.000000,1.000000" _scalevalue)))
        (:then_2
          (Transformation|SetRelativeRotation (Variables|Default|GetTurretMesh) (Math|Rotator|MakeRotator 0.0 (.y (Math|Vector|Lerp(Vector) "0.000000,360.000000,0.000000" "1.000000,1.000000,1.000000" _scalevalue)) 0.0) false false))))))

(event Custom|EventOnReversAnimDeactivation
  (bind _scalevalue (Timeline|ScalingWeapon Reverse)
    (:Update
      (Utilities|FlowControl|Sequence
        (:then_0
          (Transformation|SetWorldScale3D (Variables|Default|GetSphereDetectedCollision) (Math|Vector|Lerp(Vector) "0, 0, 0" "30.000000,30.000000,30.000000" _scalevalue)))
        (:then_1
          (Transformation|SetWorldScale3D (Variables|Default|GetTurretMesh) (Math|Vector|Lerp(Vector) "0, 0, 0" "1.000000,1.000000,1.000000" _scalevalue))
          (Variables|Default|SetCurrentScale (Math|Vector|Lerp(Vector) "0, 0, 0" "1.000000,1.000000,1.000000" _scalevalue)))
        (:then_2
          (Transformation|SetRelativeRotation (Variables|Default|GetTurretMesh) (Math|Rotator|MakeRotator 0.0 (.y (Math|Vector|Lerp(Vector) "0.000000,360.000000,0.000000" "1.000000,1.000000,1.000000" _scalevalue)) 0.0) false false))))))

(event EventBeginPlay
  (Utilities|FlowControl|Sequence
    (:then_0
      (bind _returnvalue (Utilities|Time|SetTimerbyEvent (EventDispatchers|CreateEvent :!event Custom|EventOnLookToTarget) 0.01 true))
      (bind _output_get (Variables|Default|SetControllerLookToTarget _returnvalue))
      (Utilities|Time|PauseTimerbyHandle _output_get))
    (:then_1
      (bind _returnvalue_2 (Utilities|Time|SetTimerbyEvent (EventDispatchers|CreateEvent :!event Custom|EventOnLineTrace) 0.01 true))
      (bind _output_get_2 (Variables|Default|SetControllerLineTrace _returnvalue_2))
      (Utilities|Time|PauseTimerbyHandle _output_get_2))
    (:then_2
      (bind _returnvalue_3 (Utilities|Time|SetTimerbyEvent (EventDispatchers|CreateEvent :!event Custom|EventOnShoot) 0.1 true))
      (bind _output_get_3 (Variables|Default|SetControllerShoot _returnvalue_3))
      (Utilities|Time|PauseTimerbyHandle _output_get_3))
    (:then_3)))

(event EventDeactivate
  (CallFunction|EventonReversAnimDeactivation)
  (Utilities|Time|PauseTimerbyHandle (Variables|Default|GetControllerLookToTarget))
  (Utilities|Time|PauseTimerbyHandle (Variables|Default|GetControllerLineTrace)))

(event EventActivate
  (CallFunction|EventonStartAnimActivation)
  (Utilities|Time|UnpauseTimerbyHandle (Variables|Default|GetControllerLookToTarget))
  (Utilities|Time|UnpauseTimerbyHandle (Variables|Default|GetControllerLineTrace)))

(fn ConstructionScript)

(fn GetLenchEnemysandTargetIndex
  (params (bLenchEnemys :type Boolean) (bIndexTargetAim :type Boolean))
  (bind _targetaim (Variables|Default|GetTargetAim))
  (bind _enemyes (Variables|Default|GetEnemyes))
  (bind _returnvalue (Utilities|Array|FindItem _enemyes _targetaim))
  (Utilities|FlowControl|Sequence
    (:then_0
      (if bLenchEnemys
        (bind _result (Math|Integer|DecrementInt (Utilities|Array|Length _enemyes))
          (:%20%20
            (return _result _returnvalue)))))
    (:then_1
      (if bIndexTargetAim
        (return _result _returnvalue)))))

(fn SphereorTurretVisibiliti
  (params (bVisible :type Boolean))
  (if bVisible
    (CallFunction|EventonStartAnimActivation)
    (else
      (CallFunction|EventonReversAnimDeactivation))))