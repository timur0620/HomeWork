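; Sword weapon for the player character that toggles mesh visibility and collision and performs a montage-driven stab.
; The montage's "Hit" notify runs a box trace along the blade, then branches on component tags.
; Physical objects receive an impulse, characters are launched, and both spawn a hit particle.
; Bone-tagged hits also ragdoll from the closest bone via the player character's ragdoll functions, disabled after a delay.
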(event Custom|EventOnStabSword
  (bind _notifyname (Animation|Montage|PlayMontage (Variables|Default|GetMeshCharacter) "/Game/Characters/CharactersDodgeRock/CustomAnimation/Montage/AM_StabSword.AM_StabSword" 1.5)
    (:OnNotifyBegin
      (if (== _notifyname "Hit")
        (bind _outhit (Collision|BoxTraceByChannel (Transformation|GetWorldLocation (Variables|Default|GetPointStart)) (Transformation|GetWorldLocation (Variables|Default|GetPointEmmiter)) "3.000000,3.000000,3.000000" "0, 0, 0" "TraceTypeQuery3" false 0 "ForDuration"))
        (Utilities|IsValid (.hitcomponent _outhit)
          (:Is%20Valid
            (Utilities|FlowControl|Sequence
              (:then_0
                (if (Components|ComponentHasTag (.hitcomponent _outhit) "PhysicalObject")
                  (Physics|AddImpulse (.hitcomponent _outhit) (* (.normal _outhit) -10000) "None" false)
                  (Effects|SpawnEmitteratLocation "/Game/Developers/Timur/Collections/ContentPack/FXVarietyPack/Particles/P_ky_hit1.P_ky_hit1" (Transformation|GetWorldLocation (Variables|Default|GetPointEmmiter)) "0, 0, 0" "0.300000,0.300000,0.300000" :!label _label)))
              (:then_1
                (if (Components|ComponentHasTag (.hitcomponent _outhit) "CharacterMesh")
                  (bind _ascharacter (Utilities|Casting|CastToCharacter (.hitactor _outhit)))
                  (Character|LaunchCharacter _ascharacter (* (.normal _outhit) -1000) false false)
                  (goto _label)))
              (:then_2
                (if (Components|ComponentHasTag (.hitcomponent _outhit) "CharacterBone")
                  (bind _ascharacter_2 (Utilities|Casting|CastToCharacter (.hitactor _outhit)))
                  (Character|LaunchCharacter _ascharacter_2 (* (.normal _outhit) -1000) false false)
                  (bind _meshtransform (CallFunction|StabtoBone _ascharacter_2 (.location _outhit)))
                  (Utilities|FlowControl|Sequence
                    (:then_0
                      (Utilities|FlowControl|Delay 2.0)
                      (Default|DisableRagdoll (Variables|Default|GetCharacterDodgeRock) _meshtransform true (Variables|/Script/Engine.Character|GetCapsuleComponent _ascharacter_2) (Variables|/Script/Engine.Character|GetMesh _ascharacter_2)))
                    (:then_1
                      (goto _label))))))))))))

(event EventBeginPlay
  (Utilities|FlowControl|Sequence
    (:then_0
      (bind _asbp_character_dodge_rock (Utilities|Casting|CastToBP_CharacterDodgeRock (Game|GetPlayerCharacter 0)))
      (bind _output_get (Variables|Default|SetCharacterDodgeRock _asbp_character_dodge_rock))
      (Variables|Default|SetMeshCharacter (Variables|/Script/Engine.Character|GetMesh _output_get)))))

(event EventDeactivate
  (bind _staticmeshsword (Variables|Default|GetStaticMeshSword))
  (Rendering|SetVisibility _staticmeshsword false false)
  (Collision|SetCollisionEnabled _staticmeshsword "NoCollision"))

(event EventActivate
  (bind _staticmeshsword (Variables|Default|GetStaticMeshSword))
  (Rendering|SetVisibility _staticmeshsword true false)
  (Collision|SetCollisionEnabled _staticmeshsword "QueryOnly"))

(fn ConstructionScript)

(fn StabtoBone
  (params (Character :type Character%20Object%20Reference) (LocationBone :type Vector))
  (bind _mesh (Variables|/Script/Engine.Character|GetMesh Character))
  (bind _meshtransform (Default|EnableRagdoll (Variables|Default|GetCharacterDodgeRock) true (.ReturnValue (Class|SkinnedMeshComponent|FindClosestBoneK2 _mesh LocationBone 0.0)) _mesh))
  (return _meshtransform))