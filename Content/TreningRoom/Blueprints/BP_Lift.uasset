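; BP_Lift is a training-room lift that moves along its own up vector while a player overlaps it.
; Begin and end overlap events from actors tagged Player open and close a gate on Tick.
; While the gate is open, Tick offsets the actor at 100 units per second, scaled by delta time, without sweeping.
; The file has no upper limit or return movement.
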(event Collision|EventActorBeginOverlap
  (params (OtherActor :type Actor%20Object%20Reference))
  (bind _returnvalue (Actor|ActorHasTag OtherActor "Player"))
  (if _returnvalue
    (Utilities|FlowControl|Gate _returnvalue) ; enters at Open
  ))

(event Collision|EventActorEndOverlap
  (params (OtherActor :type Actor%20Object%20Reference))
  (if (Actor|ActorHasTag OtherActor "Player")
    (Utilities|FlowControl|Gate (Actor|ActorHasTag (stale Collision|EventActorBeginOverlap OtherActor) "Player")) ; enters at Close
  ))

(event EventTick
  (params (DeltaSeconds :type Float%20%28single-precision%29))
  (Utilities|IsValid (stale Collision|EventActorBeginOverlap OtherActor)
    (:Is%20Valid
      (Utilities|FlowControl|Gate (Actor|ActorHasTag (stale Collision|EventActorBeginOverlap OtherActor) "Player")
        (:Exit
          (Transformation|AddActorWorldOffset (* (* (Transformation|GetActorUpVector) (Utilities|Time|GetWorldDeltaSeconds)) 1e+02)))))))

(fn ConstructionScript)