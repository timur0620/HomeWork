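; Game mode for DodgeRock that drives the start, rock spawning, game over and restart of a rock-dodging game.
; BeginPlay caches and starts the game state, then binds to the player character health component's owner-death event to end the game.
; Process takes a time value and, on multiples of five, has the level's rock spawner spawn a rock and increments the game state's rock count.
; Start, end and restart logic is delegated to BP_GameStateDodgeRock.
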(event Custom|Process
  (params (CurrentTime :type Integer))
  (if (== (Math|Integer|%(Integer) CurrentTime 5) 0)
    (CallFunction|SpawnRock)
    (bind _gamestatebasedodgerock (Variables|Default|GetGameStateBaseDodgeRock)
      (:then
        (bind _result (Math|Integer|IncrementInt (Default|GetRockCount _gamestatebasedodgerock))
          (:%20%20
            (Default|SetRockCount _gamestatebasedodgerock _result))))
      (:else))))

(event Custom|SpawnRock
  (bind _returnvalue (Actor|GetActorOfClass "/Game/DodgeRock/Gameplay/Spawners/BP_RockSpawner.BP_RockSpawner_C"))
  (Default|SpawnRockinVolume _returnvalue))

(event Custom|EndGame
  (bind _gamestatebasedodgerock (Variables|Default|GetGameStateBaseDodgeRock)
    (:then
      (Default|EndGameGSDR _gamestatebasedodgerock))
    (:else)))

(event Custom|RestartGame
  (bind _gamestatebasedodgerock (Variables|Default|GetGameStateBaseDodgeRock)
    (:then
      (Default|RestartGameGSDR _gamestatebasedodgerock))
    (:else)))

(event Custom|OnPlayerDead
  (CallFunction|EndGame))

(event EventBeginPlay
  ;[1 1 1] Init
  (Utilities|FlowControl|Sequence
    (:then_0
      (bind _asbp_game_state_dodge_rock (Utilities|Casting|CastToBP_GameStateDodgeRock (Game|GetGameState)))
      (bind _output_get (Variables|Default|SetGameStateBaseDodgeRock _asbp_game_state_dodge_rock))
      (Default|StartGameGSDR _output_get))
    (:then_1
      (bind _asbp_character_dodge_rock (Utilities|Casting|CastToBP_CharacterDodgeRock (Game|Player|GetPlayerPawn 0)))
      (bind _output_get_2 (Variables|Default|SetDodgeRockPlayerCharacters _asbp_character_dodge_rock))
      (EventDispatchers|BindEventtoOnOwnerDead (Variables|/Game/Characters/CharactersDodgeRock/BP_CharacterDodgeRock.BP_CharacterDodgeRock_C|GetBP_HealthComponents _output_get_2) (EventDispatchers|CreateEvent :!event Custom|OnPlayerDead)))))

(fn ConstructionScript)