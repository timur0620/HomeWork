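; Game state for DodgeRock that runs the match timer, scoring and save/load, and initializes coins and the turret.
; A one-second timer adds the rock count to the player's score and passes elapsed time to the game mode.
; Game end records the score in the game instance and triggers a delayed restart.
; Saving stores bonus count and coin actors, then quits; loading destroys coins missing from the save.
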(event Custom|EndGameGSDR
  (Utilities|Time|ClearandInvalidateTimerbyHandle (Variables|Default|GetCoreGameTime))
  (Variables|Default|SetIsGameEnded true)
  (Utilities|FlowControl|Sequence
    (:then_0
      (bind _asbp_game_instance_dodge_rock (Utilities|Casting|CastToBP_GameInstanceDodgeRock (Game|GetGameInstance)))
      (bind _playerstatedodgerock (Variables|Default|GetPlayerStateDodgeRock)
        (:then
          (Default|SetHighestScore _asbp_game_instance_dodge_rock (Default|GetPlayerScore _playerstatedodgerock)))
        (:else)))
    (:then_1
      (Utilities|FlowControl|Delay 3.0)
      (bind _gamemodsdodgerock (Variables|Default|GetGameModsDodgeRock)
        (:then
          (Default|RestartGame _gamemodsdodgerock))
        (:else)))))

(event Custom|RestartGameGSDR
  (bind _returnvalue (Game|GetCurrentLevelName true))
  (Game|OpenLevel(byName) (Utilities|String|StringToName _returnvalue)))

(event Custom|StartGameGSDR
  (bind _returnvalue (Utilities|Time|SetTimerbyEvent (EventDispatchers|CreateEvent :!event Custom|CoreGameTimeEvent) 1.0 true))
  (Variables|Default|SetCoreGameTime _returnvalue)
  (Variables|Default|SetIsGameEnded false))

(event Custom|CoreGameTimeEvent
  (bind _result (Math|Integer|IncrementInt (Variables|Default|GetTimePlayed))
    (:%20%20
      (Variables|Default|SetTimePlayed _result)
      (Utilities|FlowControl|Sequence
        (:then_0
          (bind _playerstatedodgerock (Variables|Default|GetPlayerStateDodgeRock)
            (:then
              (Default|SetPlayerScore _playerstatedodgerock (+ (Default|GetPlayerScore _playerstatedodgerock) (CallFunction|GetRockCount))))
            (:else)))
        (:then_1
          (bind _gamemodsdodgerock (Variables|Default|GetGameModsDodgeRock)
            (:then
              (Default|Process _gamemodsdodgerock (Variables|Default|GetTimePlayed)))
            (:else)))))))

(event Custom|SaveGameEvent
  (bind _returnvalue (SaveGame|CreateSaveGameObject "/Game/TreningRoom/SaveGame/BP_SaveCoin.BP_SaveCoin_C"))
  (Variables|/Game/TreningRoom/SaveGame/BP_SaveCoin.BP_SaveCoin_C|SetSaveCounterBonus _returnvalue (Variables|/Game/DodgeRock/Core/GameInstance/BP_GameInstanceDodgeRock.BP_GameInstanceDodgeRock_C|GetCurrentCounterBonus (Variables|Default|GetGameInstanceDodgeRock)))
  (bind _outactors (Actor|GetAllActorsOfClass "/Game/TreningRoom/Blueprints/BP_Coin.BP_Coin_C"))
  (Variables|/Game/TreningRoom/SaveGame/BP_SaveCoin.BP_SaveCoin_C|SetBonusCoinsOnLevel _returnvalue _outactors)
  (SaveGame|SaveGametoSlot _returnvalue "CountAndCoins")
  (Development|PrintString "GAME   SAVED 
")
  (Game|QuitGame 0 "Quit" false))

(event Custom|LoadGameEvent
  (bind _returnvalue (SaveGame|LoadGamefromSlot "CountAndCoins"))
  (bind _asbp_save_coin (Utilities|Casting|CastToBP_SaveCoin _returnvalue))
  (Variables|/Game/DodgeRock/Core/GameInstance/BP_GameInstanceDodgeRock.BP_GameInstanceDodgeRock_C|SetCurrentCounterBonus (Variables|Default|GetGameInstanceDodgeRock) (Variables|/Game/TreningRoom/SaveGame/BP_SaveCoin.BP_SaveCoin_C|GetSaveCounterBonus _asbp_save_coin))
  (bind _outactors (Actor|GetAllActorsOfClass "/Game/TreningRoom/Blueprints/BP_Coin.BP_Coin_C"))
  (if (> (Utilities|Array|Length _outactors) 0)
    (Development|PrintString "GAME   LOADED 
")
    (for _array_element _outactors
      (if (not (Utilities|Array|ContainsItem (Variables|/Game/TreningRoom/SaveGame/BP_SaveCoin.BP_SaveCoin_C|GetBonusCoinsOnLevel _asbp_save_coin) _array_element))
        (Actor|DestroyActor _array_element)))))

(event EventBeginPlay
  (Utilities|FlowControl|Sequence
    (:then_0
      (bind _asbp_game_mods_dodge_rock (Utilities|Casting|CastToBP_GameModsDodgeRock (Game|GetGameMode)))
      (Variables|Default|SetGameModsDodgeRock _asbp_game_mods_dodge_rock))
    (:then_1
      (bind _asbp_player_state_dodge_rock (Utilities|Casting|CastToBP_PlayerStateDodgeRock (Game|GetPlayerState 0)))
      (Variables|Default|SetPlayerStateDodgeRock _asbp_player_state_dodge_rock))
    (:then_2
      (bind _outactors (Actor|GetAllActorswithInterface "/Game/DodgeRock/Blueprints/Interfaces/BPI_Init.BPI_Init_C"))
      (bind _array_element (Utilities|Array|ForEachLoopwithBreak _outactors :!label _label)
        (:LoopBody
          (bind _asbp_coin (Utilities|Casting|CastToBP_Coin _array_element))
          (Utilities|FlowControl|DoOnce false
            (:Completed
              (Default|Init _asbp_coin))))
        (:Completed
          (bind _asbp_turret_dodge_rock (Utilities|Casting|CastToBP_TurretDodgeRock _array_element))
          (Default|Init _asbp_turret_dodge_rock)
          (goto _label Break))))
    (:then_3
      (EventDispatchers|BindEventtoOnSaveGame (EventDispatchers|CreateEvent :!event Custom|SaveGameEvent))
      (EventDispatchers|BindEventtoOnLoadGame (EventDispatchers|CreateEvent :!event Custom|LoadGameEvent)))
    (:then_4
      (bind _asbp_game_instance_dodge_rock (Utilities|Casting|CastToBP_GameInstanceDodgeRock (Game|GetGameInstance)))
      (Variables|Default|SetGameInstanceDodgeRock _asbp_game_instance_dodge_rock))))

(fn ConstructionScript)

(fn GetRockCount
  (return (Variables|Default|GetRockCount)))

(fn SetRockCount
  (params (RockCount :type Integer))
  (bind _output_get (Variables|Default|SetRockCount RockCount))
  (return _output_get))