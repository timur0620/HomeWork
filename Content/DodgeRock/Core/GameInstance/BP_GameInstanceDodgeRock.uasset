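; Game Instance Blueprint for DodgeRock that holds the game difficulty and highest score for the running game session.
; Simple getter and setter functions expose both values, with each setter storing its input and returning it.
; The setters assign values directly, with no high-score comparison or save-to-disk logic.
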(fn GetGameDifficulty
  (return (Variables|Default|GetGameDifficulty)))

(fn SetGameDificulty
  (params (GameDifficulty :type EGameDifficulty%20Enum :default "NewEnumerator0"))
  (bind _output_get (Variables|Default|SetGameDifficulty GameDifficulty))
  (return _output_get))

(fn GetHighestScore
  (return (Variables|Default|GetHighestScore)))

(fn SetHighestScore
  (params (HighestScore :type Integer))
  (bind _output_get (Variables|Default|SetHighestScore HighestScore))
  (return _output_get))