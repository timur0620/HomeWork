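; Short-lived projectile for a turret that damages actors tagged Enemy.
; On sphere overlap with an enemy it applies damage, spawns a hit particle and reveals a hit widget, while other actors get a different particle.
; Any valid hit, or an end overlap, stops projectile movement and disables collision.
; The bullet never destroys itself on impact, relying on a brief lifespan set at BeginPlay for cleanup.
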(event OnComponentBeginOverlap(SphereMainCollision)
  (params (OverlappedComponent :type Primitive%20Component%20Object%20Reference) (OtherActor :type Actor%20Object%20Reference) (OtherComp :type Primitive%20Component%20Object%20Reference) (OtherBodyIndex :type Integer) (bFromSweep :type Boolean) (SweepResult :type Hit%20Result%20Structure%20%28by%20ref%29))
  (bind _returnvalue (Transformation|GetActorLocation))
  (Utilities|IsValid OtherActor
    (:Is%20Valid
      (if (Actor|ActorHasTag OtherActor "Enemy")
        (Effects|SpawnEmitteratLocation "/Game/Developers/Timur/Collections/ContentPack/FXVarietyPack/Particles/P_ky_hit1.P_ky_hit1" _returnvalue "0, 0, 0" "0.300000,0.300000,0.300000")
        (Game|Damage|ApplyDamage OtherActor (Variables|Components|GetDamage) 0 self)
        (Rendering|SetVisibility (Variables|Default|GetWidgetMainHit) true false)
        (Variables|/Script/Engine.ProjectileMovementComponent|SetbSimulationEnabled (Variables|Default|GetProjectileMovementMain) false)
        (Collision|SetCollisionEnabled (Variables|Default|GetSphereMainCollision) "NoCollision")
        (else
          (Effects|SpawnEmitteratLocation "/Game/Developers/Timur/Collections/ContentPack/FXVarietyPack/Particles/P_ky_hit2.P_ky_hit2" _returnvalue "0, 0, 0" "0.300000,0.300000,0.300000")
          (Variables|/Script/Engine.ProjectileMovementComponent|SetbSimulationEnabled (Variables|Default|GetProjectileMovementMain) false)
          (Collision|SetCollisionEnabled (Variables|Default|GetSphereMainCollision) "NoCollision"))))))

(event OnComponentEndOverlap(SphereMainCollision)
  (params (OverlappedComponent :type Primitive%20Component%20Object%20Reference) (OtherActor :type Actor%20Object%20Reference) (OtherComp :type Primitive%20Component%20Object%20Reference) (OtherBodyIndex :type Integer))
  (Variables|/Script/Engine.ProjectileMovementComponent|SetbSimulationEnabled (Variables|Default|GetProjectileMovementMain) false)
  (Collision|SetCollisionEnabled (Variables|Default|GetSphereMainCollision) "NoCollision"))

(event EventBeginPlay
  (Actor|SetLifeSpan 0.5)
  (Rendering|SetVisibility (Variables|Default|GetWidgetMainHit) false false))

(fn ConstructionScript)