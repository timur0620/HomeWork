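; BP_TriggerDeadPlayer is a DodgeRock trigger actor that deals lethal damage to the player on overlap.
; On BeginPlay it binds its actor begin-overlap event and caches the health component from the player character.
; When an actor tagged Player overlaps, it applies damage equal to twice that component's default health, naming itself as the damage causer.
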(event Custom|OnActorOverlap_Event
  (params (OverlappedActor :type Actor%20Object%20Reference) (OtherActor :type Actor%20Object%20Reference))
  (if (Actor|ActorHasTag OtherActor "Player")
    (Game|Damage|ApplyDamage OtherActor (* (Default|GetDefaultHealth (Variables|Default|Get%20HealthComponents)) 2.0) 0 self)))

(event EventBeginPlay
  (Collision|BindEventtoOnActorBeginOverlap (EventDispatchers|CreateEvent :!event Custom|OnActorOverlap_Event))
  (bind _asbp_character_dodge_rock (Utilities|Casting|CastToBP_CharacterDodgeRock (Game|GetPlayerCharacter 0)))
  (Variables|Default|Set%20HealthComponents (Variables|/Game/Characters/CharactersDodgeRock/BP_CharacterDodgeRock.BP_CharacterDodgeRock_C|GetBP_HealthComponents _asbp_character_dodge_rock)))

(fn ConstructionScript)