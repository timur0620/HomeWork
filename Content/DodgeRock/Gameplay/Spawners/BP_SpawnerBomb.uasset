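; BP_SpawnerBomb is a DodgeRock spawner that periodically creates AI bomb enemies inside a box area.
; A looping timer set on BeginPlay drives spawning, gated by the GetLengthArrayBombInScene check.
; Each enemy spawns at a random X/Y within the collision box at the spawner's Z, with an emitter effect.
; Valid spawns register in the cached game state's BombsInScene array.
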(event Custom|SpawnBombEnemy_Event
  (bind _gamestatedodgerock (Variables|Default|GetGameStateDodgeRock))
  (if (Utilities|GetLengthArrayBombinScene)
    (bind _returnvalue (AI|SpawnAIFromClass "/Game/DodgeRock/Gameplay/Characters/Enemies/BP_CharacterBombEnemy.BP_CharacterBombEnemy_C" 0 (CallFunction|GetPointtoBoxFunction (Variables|Default|GetBoxCollision)) "0, 0, 0" false 0))
    (Utilities|IsValid _gamestatedodgerock
      (:Is%20Valid
        (Utilities|IsValid _returnvalue
          (:Is%20Valid
            (Effects|SpawnEmitteratLocation 0 (Transformation|GetActorLocation _returnvalue))
            (Utilities|Array|AddUnique (Variables|/Game/DodgeRock/Core/GameState/BP_GameStateDodgeRock.BP_GameStateDodgeRock_C|GetBombsInScene _gamestatedodgerock) _returnvalue)))))))

(event EventBeginPlay
  (Utilities|FlowControl|Sequence
    (:then_0
      (Utilities|Time|SetTimerbyEvent (EventDispatchers|CreateEvent :!event Custom|SpawnBombEnemy_Event) (Variables|Default|GetIntervalSpawn) true))
    (:then_1
      (bind _asbp_game_state_dodge_rock (Utilities|Casting|CastToBP_GameStateDodgeRock (Game|GetGameState)))
      (Variables|Default|SetGameStateDodgeRock _asbp_game_state_dodge_rock))))

(fn ConstructionScript)

(fn GetPointtoBoxFunction
  (params (CollisionBox :type Box%20Component%20Object%20Reference))
  (bind _returnvalue (Transformation|GetWorldLocation CollisionBox))
  (bind _returnvalue_2 (Components|Box|GetScaledBoxExtent CollisionBox))
  (bind _returnvalue_3 (Math|Random|RandomPointinBoundingBox _returnvalue _returnvalue_2))
  (bind (_x _y) (Math|Vector|BreakVector _returnvalue_3))
  (return (Math|Vector|MakeVector _x _y (.Z (Math|Vector|BreakVector (Transformation|GetActorLocation))))))