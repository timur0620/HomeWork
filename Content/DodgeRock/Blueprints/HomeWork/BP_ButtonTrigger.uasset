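; BP_ButtonTrigger is an interaction trigger for DodgeRock that lets the player switch all BPI_Switchable actors on and off with the E key.
; Tagged-player overlap binds or unbinds the character's OnPressE, toggles the HUD's flashing E prompt and shows or hides an info panel, gated by paired DoOnce nodes.
; A looping timer, paused while the panel is hidden, yaws it toward the player within a clamped range.
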(event Custom|SwitchEvent
  (Utilities|FlowControl|FlipFlop
    (:A
      (bind _outactors (Utilities|IterInterface)
        (:LoopBody
          (Class|BPISwitchable|Swithon(Message) _outactors))))
    (:B
      (bind _outactors_2 (Utilities|IterInterface)
        (:LoopBody
          (Class|BPISwitchable|SwitchOff(Message) _outactors_2))))))

(event Custom|OnLookAtToPlayer_Event
  (Transformation|SetWorldRotation (Variables|Default|GetInfoWidget) (Math|Rotator|MakeRotator 0.0 0.0 (Math|Float|Clamp(Float) (.yaw (Math|Rotator|FindLookatRotation (Transformation|GetWorldLocation (Variables|Default|GetInfoWidget)) (Transformation|GetActorLocation (Game|GetPlayerCharacter 0)))) 15.0 1e+02)) false false))

(event Collision|EventActorBeginOverlap
  (params (OtherActor :type Actor%20Object%20Reference))
  (if (Actor|ActorHasTag OtherActor "Player")
    (Utilities|FlowControl|DoOnce false
      (:Completed
        (EventDispatchers|BindEventtoOnPressE (Variables|Default|GetCharacterDodgeRock) (EventDispatchers|CreateEvent :!event Custom|SwitchEvent))
        (bind _playerinterfacewidget (Utilities|GetPlayerInterface))
        (Default|StartFlashingButtonEEvent _playerinterfacewidget)
        (CallFunction|InfoPanelController false)
        (Utilities|FlowControl|DoOnce false) ; enters at Reset
      ))))

(event EventBeginPlay
  (Utilities|FlowControl|Sequence
    (:then_0
      (bind _asbp_character_dodge_rock (Utilities|Casting|CastToBP_CharacterDodgeRock (Game|GetPlayerCharacter 0)))
      (Variables|Default|SetCharacterDodgeRock _asbp_character_dodge_rock))
    (:then_1
      (bind _returnvalue (Utilities|Time|SetTimerbyEvent (EventDispatchers|CreateEvent :!event Custom|OnLookAtToPlayer_Event) 0.05 true))
      (Variables|Default|SetTimerLookInfoPanel _returnvalue))
    (:then_2
      (CallFunction|InfoPanelController true))
    (:then_3
      (Variables|Default|SetCurrentScale (Transformation|GetWorldScale (Variables|Default|GetInfoWidget))))))

(event Collision|EventActorEndOverlap
  (params (OtherActor :type Actor%20Object%20Reference))
  (if (Actor|ActorHasTag OtherActor "Player")
    (Utilities|FlowControl|DoOnce false
      (:Completed
        (EventDispatchers|UnbindallEventsfromOnPressE (Variables|Default|GetCharacterDodgeRock))
        (bind _playerinterfacewidget (Utilities|GetPlayerInterface))
        (Default|StopFlafhingButtonEEvent _playerinterfacewidget)
        (CallFunction|InfoPanelController true)
        (Utilities|FlowControl|DoOnce false) ; enters at Reset
      ))))

(fn ConstructionScript)

(fn InfoPanelController
  (params (bNewVisibility :type Boolean))
  (if bNewVisibility
    (Rendering|SetVisibility (Variables|Default|GetInfoWidget) false false)
    (Utilities|Time|PauseTimerbyHandle (Variables|Default|GetTimerLookInfoPanel))
    (else
      (Rendering|SetVisibility (Variables|Default|GetInfoWidget) true false)
      (Utilities|Time|UnpauseTimerbyHandle (Variables|Default|GetTimerLookInfoPanel)))))