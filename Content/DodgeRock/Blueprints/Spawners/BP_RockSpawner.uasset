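; Rock spawner actor for DodgeRock that drops BP_Rock hazards into a box volume, with damage scaled to game difficulty.
; On BeginPlay it reads the difficulty from the game instance and selects the base rock damage.
; The SpawnRockInVolume event spawns a rock at a random X/Y inside the box, at the spawner's own height, and passes it that damage.
; The file contains no timer or call that triggers spawning.
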(event Custom|SpawnRockInVolume
  (bind _boxcollision (Variables|Default|GetBoxCollision))
  (bind _returnvalue (Transformation|GetWorldLocation _boxcollision))
  (bind _returnvalue_2 (Components|Box|GetScaledBoxExtent _boxcollision))
  (bind _returnvalue_3 (Math|Random|RandomPointinBoundingBox _returnvalue _returnvalue_2))
  (bind (_x _y) (Math|Vector|BreakVector _returnvalue_3))
  (Game|SpawnActorfromClass "/Game/DodgeRock/Blueprints/BP_Rock.BP_Rock_C" (Math|Transform|MakeTransform (Math|Vector|MakeVector _x _y (.Z (Math|Vector|BreakVector (Transformation|GetActorLocation))))) "AdjustIfPossibleButAlwaysSpawn" 0 (Variables|Default|GetBaseRockDamege) 0))

(event EventBeginPlay
  (bind _asbp_game_instance_dodge_rock (Utilities|Casting|CastToBP_GameInstanceDodgeRock (Game|GetGameInstance)))
  (Variables|Default|SetBaseRockDamege (Utilities|Select :Index (Default|GetGameDifficulty _asbp_game_instance_dodge_rock) :NewEnumerator0 25.0 :NewEnumerator1 5e+01 :NewEnumerator2 1e+02)))

(fn ConstructionScript)