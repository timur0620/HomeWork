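; Bomb enemy character for DodgeRock that chases the player and explodes on reaching them.
; BeginPlay starts a looping one-second timer, apparently driving the chase event, and caches the DodgeRock game state.
; The chase uses AI MoveTo toward the player; on success it spawns an explosion and applies damage.
; It then removes itself from the game state's BombsInScene list and destroys itself.
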(event Custom|ChasePlayer_Event
  (bind _self self)
  (AI|AIMoveTo self "0, 0, 0" (Game|GetPlayerCharacter 0) 1e+02 true
    (:OnSuccess
      (Effects|SpawnEmitteratLocation "/Game/StarterContent/Particles/P_Explosion.P_Explosion" (Transformation|GetActorLocation))
      (Game|Damage|ApplyDamage (Game|GetPlayerCharacter 0) (Variables|Default|GetBase%20Damage) 0 self)
      (Utilities|IsValid _self
        (:Is%20Valid
          (Utilities|Array|RemoveItem (Variables|/Game/DodgeRock/Core/GameState/BP_GameStateDodgeRock.BP_GameStateDodgeRock_C|GetBombsInScene (Variables|Default|GetGameStateDodgeRock)) self)
          (Actor|DestroyActor _self))))))

(event EventBeginPlay
  (Utilities|FlowControl|Sequence
    (:then_0
      (Utilities|Time|SetTimerbyEvent (EventDispatchers|CreateEvent :!event Custom|ChasePlayer_Event) 1.0 true))
    (:then_1
      (bind _asbp_game_state_dodge_rock (Utilities|Casting|CastToBP_GameStateDodgeRock (Game|GetGameState)))
      (Variables|Default|SetGameStateDodgeRock _asbp_game_state_dodge_rock))))

(fn ConstructionScript)