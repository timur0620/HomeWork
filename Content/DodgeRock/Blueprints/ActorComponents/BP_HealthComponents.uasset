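; Actor component that tracks its owner's health and signals when it runs out.
; On BeginPlay it binds to the owner's OnTakeAnyDamage, then subtracts incoming damage, clamped between zero and current health.
; At zero it calls OnOwnerDead, with no guard against repeat calls on later hits.
; Both the Health and DefaultHealth accessors use the single DefaultHealth variable, so the starting value is not preserved.
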(event Custom|OnTakeAnyDamage_Event
  (params (DamagedActor :type Actor%20Object%20Reference) (Damage :type Float%20%28single-precision%29) (DamageType :type Damage%20Type%20Object%20Reference) (InstigatedBy :type Controller%20Object%20Reference) (DamageCauser :type Actor%20Object%20Reference))
  (bind _defaulthealth (CallFunction|GetHealth))
  (CallFunction|SetHealth (Math|Float|Clamp(Float) (- _defaulthealth Damage) 0.0 _defaulthealth))
  (if (<= (CallFunction|GetHealth) 0.0)
    (Default|CallOnOwnerDead)))

(event EventBeginPlay
  (EventDispatchers|AssignOnTakeAnyDamage (Components|GetOwner) (EventDispatchers|CreateEvent :!event Custom|OnTakeAnyDamage_Event))
  (CallFunction|SetHealth (Variables|Default|GetDefaultHealth)))

(fn GetHealth
  (return (Variables|Default|GetDefaultHealth)))

(fn SetHealth
  (params (DefaultHealth :type Float%20%28double-precision%29))
  (bind _output_get (Variables|Default|SetDefaultHealth DefaultHealth))
  (return _output_get))

(fn GetDefaultHealth
  (return (Variables|Default|GetDefaultHealth)))

(fn SetDefaultHealth
  (params (DefaultHealth :type Float%20%28double-precision%29))
  (bind _output_get (Variables|Default|SetDefaultHealth DefaultHealth))
  (return _output_get))