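; BP_TriggerShootTurretSwitch is a DodgeRock box trigger that starts or stops firing on a turret chosen by IndexTurret.
; With IsStart set, it swaps its mesh to DiscMaterial on BeginPlay and starts firing when a Player-tagged actor overlaps.
; Otherwise any overlapping actor stops firing, with no tag check.
; FindRefIndex resolves the turret through MapTurretsToScene on BP_GameStateDodgeRock.
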(event OnComponentBeginOverlap(BoxTrigger)
  (params (OverlappedComponent :type Primitive%20Component%20Object%20Reference) (OtherActor :type Actor%20Object%20Reference) (OtherComp :type Primitive%20Component%20Object%20Reference) (OtherBodyIndex :type Integer) (bFromSweep :type Boolean) (SweepResult :type Hit%20Result%20Structure%20%28by%20ref%29))
  (if (Variables|Default|GetIsStart?)
    (if (Actor|ActorHasTag OtherActor "Player")
      (bind _output (Utilities|FindRefIndex))
      (Default|StartFireEvent _output))
    (else
      (Default|StopFireEvent _output))))

(event EventBeginPlay
  (bind _asbp_game_state_dodge_rock (Utilities|Casting|CastToBP_GameStateDodgeRock (Game|GetGameState)))
  (Variables|Default|SetGameStateDodgeRock _asbp_game_state_dodge_rock)
  (if (Variables|Default|GetIsStart?)
    (Rendering|Material|SetMaterial (Variables|Default|GetStaticMesh) 0 "/Engine/VREditor/UI/DiscMaterial.DiscMaterial")))

(fn ConstructionScript)