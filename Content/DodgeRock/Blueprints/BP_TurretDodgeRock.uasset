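; Dodge Rock turret that turns its mesh toward the player every tick and fires BP_BulletTurret projectiles with an explosion effect.
; A looping fire timer sets the shot rate, while a second timer toggles it on and off to create bursts.
; Start/stop events pause or resume both timers.
; Init assigns IDs to all turrets and registers them in the GameState's turret map.
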(event Custom|InstantiateBullet_Event
  (bind _sc_pointinstantiate (Variables|Default|GetSC_PointInstantiate)
    (:then
      (Game|SpawnActorfromClass "/Game/DodgeRock/Blueprints/BP_BulletTurret.BP_BulletTurret_C" (Transformation|GetWorldTransform _sc_pointinstantiate) "AdjustIfPossibleButAlwaysSpawn" 0 1.0 0)
      (Effects|SpawnEmitteratLocation "/Game/ContentPack/StarterContent/Particles/P_Explosion.P_Explosion" (Transformation|GetActorLocation) "0, 0, 0" "0.200000,0.200000,0.200000"))
    (:else)))

(event Custom|StopFire_Event
  (Utilities|Time|PauseTimerbyHandle (Variables|Default|GetDelayTimerHandle))
  (Utilities|Time|PauseTimerbyHandle (Variables|Default|GetFireTimerHandle)))

(event Custom|StartFire_Event
  (Utilities|Time|UnpauseTimerbyHandle (Variables|Default|GetDelayTimerHandle))
  (Utilities|Time|UnpauseTimerbyHandle (Variables|Default|GetFireTimerHandle)))

(event EventBeginPlay
  (Utilities|FlowControl|Sequence
    (:then_0
      (bind _returnvalue (Utilities|Time|SetTimerbyEvent (EventDispatchers|CreateEvent :!event Custom|InstantiateBullet_Event) (/ 0.5 (Variables|Default|GetBulletsPerSecond)) true))
      (Variables|Default|SetFireTimerHandle _returnvalue)
      (bind _returnvalue_2 (Utilities|Time|SetTimerbyFunctionName 0 "ProsessFireFunction" (Variables|Default|GetSecDelayShoot) true))
      (Variables|Default|SetDelayTimerHandle _returnvalue_2)
      (CallFunction|StopFireEvent))
    (:then_1
      (bind _asbp_game_state_dodge_rock (Utilities|Casting|CastToBP_GameStateDodgeRock (Game|GetGameState)))
      (Variables|Default|SetGameStateDodgeRock _asbp_game_state_dodge_rock))))

(event EventTick
  (params (DeltaSeconds :type Float%20%28single-precision%29))
  ;[1 1 1] LookAtToPlayer
  (Utilities|FlowControl|Sequence
    (:then_0
      (Transformation|SetWorldRotation (Variables|Default|GetStaticMesh) (Math|Rotator|FindLookatRotation (Transformation|GetActorLocation self) (Transformation|GetActorLocation (Game|GetPlayerCharacter 0))) false false))))

(event EventInit
  (bind _outactors (Actor|GetAllActorsOfClass "BP_TurretDodgeRock_C"))
  (bind (_array_element _array_index) (Utilities|Array|ForEachLoopwithBreak _outactors)
    (:LoopBody
      (Utilities|Map|Add (Variables|/Game/DodgeRock/Core/GameState/BP_GameStateDodgeRock.BP_GameStateDodgeRock_C|GetMapTurretsToScene (Variables|Default|GetGameStateDodgeRock)) _array_index (Utilities|Struct|MakeST_TurretInfo _array_index (Class|HeadMountedDisplayFunctionLibrary|GetHMDDeviceName) (Class|KismetMathLibrary|GetDate (Class|KismetMathLibrary|Today)) _array_element (Transformation|GetActorTransform) _outactors))
      (Variables|BP_TurretDodgeRock_C|SetID _array_element _array_index))))

(fn ConstructionScript)

(fn ProsessFireFunction
  (bind _firetimerhandle (Variables|Default|GetFireTimerHandle))
  (if (Variables|Default|GetIsFire?)
    (Utilities|Time|PauseTimerbyHandle _firetimerhandle)
    (Variables|Default|SetIsFire? false)
    (else
      (Utilities|Time|UnpauseTimerbyHandle _firetimerhandle)
      (Variables|Default|SetIsFire? true))))