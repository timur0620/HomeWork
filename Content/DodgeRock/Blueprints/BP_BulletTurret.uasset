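; BP_BulletTurret is a short-lived bullet actor, apparently for a turret, that damages actors tagged Player.
; A sphere overlap with the player spawns a half-scale explosion, applies damage and destroys the bullet.
; Other overlaps spawn a full-scale explosion without damage or immediate destruction.
; The bullet is also destroyed when any overlap ends or its brief lifespan, set at BeginPlay, expires.
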(event OnComponentBeginOverlap(BulletSphereCollision)
  (params (OverlappedComponent :type Primitive%20Component%20Object%20Reference) (OtherActor :type Actor%20Object%20Reference) (OtherComp :type Primitive%20Component%20Object%20Reference) (OtherBodyIndex :type Integer) (bFromSweep :type Boolean) (SweepResult :type Hit%20Result%20Structure%20%28by%20ref%29))
  (bind _returnvalue (Transformation|GetActorLocation))
  (bind _self self)
  (if (Actor|ActorHasTag OtherActor "Player")
    (Effects|SpawnEmitteratLocation "/Game/ContentPack/StarterContent/Particles/P_Explosion.P_Explosion" _returnvalue "0, 0, 0" "0.500000,0.500000,0.500000")
    (Game|Damage|ApplyDamage OtherActor (Variables|Components|GetBaseDamage) 0 self)
    (Utilities|IsValid _self
      (:Is%20Valid
        (Actor|DestroyActor _self)))
    (else
      (Effects|SpawnEmitteratLocation "/Game/ContentPack/StarterContent/Particles/P_Explosion.P_Explosion" _returnvalue))))

(event OnComponentEndOverlap(BulletSphereCollision)
  (params (OverlappedComponent :type Primitive%20Component%20Object%20Reference) (OtherActor :type Actor%20Object%20Reference) (OtherComp :type Primitive%20Component%20Object%20Reference) (OtherBodyIndex :type Integer))
  (bind _self self)
  (Utilities|IsValid _self
    (:Is%20Valid
      (Actor|DestroyActor _self))))

(event EventBeginPlay
  (Actor|SetLifeSpan 1.5))

(fn ConstructionScript)