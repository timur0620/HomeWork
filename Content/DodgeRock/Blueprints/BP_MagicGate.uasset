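; BP_MagicGate is a gate that triggers a different effect each time the player overlaps it, cycling through a looping MultiGate.
; Effects randomize the player's material, launch the player by briefly simulating capsule physics, spawn repeated particle bursts, or toggle a spotlight green and red.
; A one-time step starts BP_Fan spinning and caches that spotlight.
; A separate Switch_Event alternates on/off messages across BPI_Switchable actors, flipping per array element.
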(event Custom|Switch_Event
  (bind _outactors (Actor|GetAllActorswithInterface "/Game/DodgeRock/Blueprints/Interfaces/BPI_Switchable.BPI_Switchable_C"))
  (for _array_element _outactors
    (Utilities|FlowControl|FlipFlop
      (:A
        (Class|BPISwitchable|Swithon(Message) _array_element))
      (:B
        (Class|BPISwitchable|SwitchOff(Message) _array_element)))))

(event Collision|EventActorBeginOverlap
  (params (OtherActor :type Actor%20Object%20Reference))
  (if (Actor|ActorHasTag OtherActor "Player")
    (Utilities|FlowControl|Sequence
      (:then_0
        (Utilities|FlowControl|MultiGate false true -1
          (:Out%200
            (Utilities|SetMaterialstoIndex (Math|Random|RandomInteger (Utilities|Array|Length (Variables|Default|GetArrayMaterials)))))
          (:Out%201
            (Utilities|ImpulsPlayertoVector "0.000000,5000.000000,0.000000"))
          (:Out%202
            (Utilities|FlowControl|DoOnce false
              (:Completed
                (bind _returnvalue (Actor|GetActorOfClass "/Game/DodgeRock/Blueprints/BP_Fan.BP_Fan_C"))
                (Variables|/Script/Engine.RotatingMovementComponent|SetRotationRate (Variables|/Game/DodgeRock/Blueprints/BP_Fan.BP_Fan_C|GetRotatingMovement _returnvalue) "180.000000,0.000000,0.000000")
                (bind _returnvalue_2 (Actor|GetActorOfClass "/Game/DodgeRock/Blueprints/BP_DoorPointLigth.BP_DoorPointLigth_C"))
                (Variables|Default|SetSpotLighth (Variables|/Game/DodgeRock/Blueprints/BP_DoorPointLigth.BP_DoorPointLigth_C|GetSpotLight _returnvalue_2)))))
          (:Out%203
            (Utilities|FlowControl|DoN 10 :!label _label
              (:Exit
                (Niagara|SpawnSystematLocation "/Niagara/DefaultAssets/Templates/Systems/DirectionalBurst.DirectionalBurst" (Transformation|GetActorLocation) "0, 0, 0" "10.000000,10.000000,10.000000")
                (Utilities|FlowControl|Delay 0.2)
                (goto _label))))
          (:Out%204
            (Utilities|FlowControl|FlipFlop
              (:A
                (Utilities|IsValid (Variables|Default|GetSpotLighth)
                  (:Is%20Valid
                    (Rendering|Components|Light|SetLightColor (Variables|Default|GetSpotLighth) "(R=0.000000,G=0.930000,B=0.237181,A=1.000000)" true))))
              (:B
                (Rendering|Components|Light|SetLightColor (Variables|Default|GetSpotLighth) "(R=0.920000,G=0.000000,B=0.277852,A=1.000000)" true)))))))))

(fn ConstructionScript)